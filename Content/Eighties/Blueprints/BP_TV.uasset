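; BP_TV is an interactive television that the player switches on and off with E while overlapping it.
; BeginPlay creates a HUD widget, which overlap shows and end overlap removes, enabling and disabling the actor's input alongside it.
; E alternates a timeline between play and reverse through a FlipFlop, fading the LED and screen glow via scalars in the DynamicTextures material parameter collection.
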(event `self.ReceiveBeginPlay`
  ;[1 1 1] HUD
  (bind _returnvalue (`|CreateWidget` "/Game/Eighties/Blueprints/Blueprint_Widget.Blueprint_Widget_C"))
  (set `self.TV_HUD` _returnvalue))

(event `self.ReceiveActorBeginOverlap`
  (params (OtherActor :type "Actor Object Reference"))
  ;[1 1 1] Trigger
  (`self.EnableInput` (`GameplayStatics.GetPlayerController` 0))
  (`UserWidget.AddToViewport` (`self.TV_HUD`) 0))

(event `Key|E`
  (params (Key :type "Key Structure"))
  ;[1 1 1] Interaction
  (:`Pressed`
    (`/Engine/EditorBlueprintResources/StandardMacros.FlipFlop`
      (:`A`
        (bind (_direction _tv_led_fade _screen_glow) (`Timeline|Timeline_0` :!label _label)
          (:`Update`
            (`KismetMaterialLibrary.SetScalarParameterValue` "/Game/Eighties/Blueprints/DynamicTextures.DynamicTextures" "LED_TV" _tv_led_fade)
            (`KismetMaterialLibrary.SetScalarParameterValue` "/Game/Eighties/Blueprints/DynamicTextures.DynamicTextures" "TV_Fade" _screen_glow))))
      (:`B`
        (goto _label :!via `Reverse`)))))

(event `self.ReceiveActorEndOverlap`
  (params (OtherActor :type "Actor Object Reference"))
  ;[1 1 1] Trigger
  (`self.DisableInput` (`GameplayStatics.GetPlayerController` 0))
  (`Widget.RemoveFromParent` (`self.TV_HUD`)))

(fn `UserConstructionScript`)