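; Interactive camera prop that takes a one-time photo when the player presses E within its overlap area.
; Overlap toggles input and a HUD widget created at BeginPlay.
; A timeline moves and rotates the ejected photo while driving fade, UV and flash emission through the DynamicTextures parameter collection, alongside a brief flashlight blink.
; PhotoTaken blocks further presses once the timeline updates, so the FlipFlop's reverse branch is effectively bypassed.
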(event `self.ReceiveBeginPlay`
  ;[1 1 1] HUD
  (set `self.Photo_taken` false)
  (bind _returnvalue (`|CreateWidget` "/Game/Eighties/Blueprints/Blueprint_Widget.Blueprint_Widget_C"))
  (set `self.Camera_HUD` _returnvalue))

(event `self.ReceiveActorBeginOverlap`
  (params (OtherActor :type "Actor Object Reference"))
  ;[1 1 1] Trigger
  (`self.EnableInput` (`GameplayStatics.GetPlayerController` 0))
  (`UserWidget.AddToViewport` (`self.Camera_HUD`) 0))

(event `Key|E`
  (params (Key :type "Key Structure"))
  (bind _flashlight (`self.Flashlight`))
  ;[1 1 1] Interaction
  (:`Pressed`
    (if (not (`self.Photo_taken`))
      (`PrimitiveComponent.CreateDynamicMaterialInstance` (`self.Photo`) 0 "/Game/Eighties/Materials/Mi_Camera_photo.Mi_Camera_photo")
      (`KismetMaterialLibrary.SetScalarParameterValue` "/Game/Eighties/Blueprints/DynamicTextures.DynamicTextures" "FlashUVs" (+ 0.0 0.5))
      (`|ExecutionSequence`
        (:`then_0`
          (`/Engine/EditorBlueprintResources/StandardMacros.FlipFlop`
            (:`A`
              (bind (_direction _rotate _photofade _photo_uvs _flash_emission _photomove) (`Timeline|Timeline_0` :!label _label)
                (:`Update`
                  (`TimelineComponent.SetPlayRate` (`self.Timeline_0`) 1.8)
                  (`SceneComponent.K2_SetRelativeLocationAndRotation` (`self.Photo`) (+ _photomove (0.0 0.0 0.0)) (`KismetMathLibrary.MakeRotator` _rotate) false false)
                  (`KismetMaterialLibrary.SetScalarParameterValue` "/Game/Eighties/Blueprints/DynamicTextures.DynamicTextures" "Photo_Fade" _photofade)
                  (`KismetMaterialLibrary.SetScalarParameterValue` "/Game/Eighties/Blueprints/DynamicTextures.DynamicTextures" "FlashUVs" _photo_uvs)
                  (`KismetMaterialLibrary.SetScalarParameterValue` "/Game/Eighties/Blueprints/DynamicTextures.DynamicTextures" "Flash_Emission" _flash_emission)
                  (set `self.Photo_taken` true))))
            (:`B`
              (goto _label :!via `Reverse`))))
        (:`then_1`
          ;[1 1 1] Flashlight
          (`SceneComponent.ToggleVisibility` _flashlight false)
          (`KismetSystemLibrary.Delay` 0.1)
          (`SceneComponent.ToggleVisibility` _flashlight false))))))

(event `self.ReceiveActorEndOverlap`
  (params (OtherActor :type "Actor Object Reference"))
  ;[1 1 1] Trigger
  (`self.DisableInput` (`GameplayStatics.GetPlayerController` 0))
  (`Widget.RemoveFromParent` (`self.Camera_HUD`)))

(fn `UserConstructionScript`)