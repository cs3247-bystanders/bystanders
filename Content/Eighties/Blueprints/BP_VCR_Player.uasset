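; Interactive VCR that shows a HUD and accepts input while an actor overlaps it, and loads a cassette on pressing E.
; E toggles the VCR light and drives an LED scalar in the DynamicTextures parameter collection through a timeline.
; Chained timelines open the housing, slide the tape in after a delay, then close the housing.
; HousingState blocks retriggering until the close finishes.
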(event `self.ReceiveBeginPlay`
  ;[1 1 1] HUD
  (set `self.HousingState` true)
  (bind _returnvalue (`|CreateWidget` "/Game/Eighties/Blueprints/Blueprint_Widget.Blueprint_Widget_C"))
  (set `self.VCR_HUD` _returnvalue))

(event `self.ReceiveActorBeginOverlap`
  (params (OtherActor :type "Actor Object Reference"))
  ;[1 1 1] Trigger
  (`self.EnableInput` (`GameplayStatics.GetPlayerController` 0))
  (`UserWidget.AddToViewport` (`self.VCR_HUD`) 0))

(event `Key|E`
  (params (Key :type "Key Structure"))
  (bind _tape (`self.Tape`))
  (bind _vcr_cassettehousing (`self.VCR_CassetteHousing`))
  ;[1 1 1] Interaction
  (:`Pressed`
    (if (`self.HousingState`)
      (`SceneComponent.ToggleVisibility` (`self.VCR_light`) false)
      ;[1 1 1] Switches LEDs on
      (`|ExecutionSequence`
        (:`then_0`
          (if (not false)
            (bind (_direction _led_on) (`Timeline|LED ON`)
              (:`Update`
                (`KismetMaterialLibrary.SetScalarParameterValue` "/Game/Eighties/Blueprints/DynamicTextures.DynamicTextures" "LED_VCR" _led_on)
                (set `self.ON State` true)))))
        (:`then_1`
          (set `self.HousingState` false)
          (bind (_direction_2 _carrigerot _led_on_2 _carriagemove) (`Timeline|HousingOpen` :!via `PlayFromStart`)
            (:`Update`
              (`|ExecutionSequence`
                (:`then_0`
                  (`SceneComponent.K2_SetRelativeLocationAndRotation` _vcr_cassettehousing (+ _carriagemove (0.0 0.0 0.0)) (`KismetMathLibrary.MakeRotator` _carrigerot) false false)
                  (`KismetSystemLibrary.Delay` 2.5)
                  (`SceneComponent.ToggleVisibility` _tape false)
                  (bind (_direction_3 _rotation _carriagemove_2) (`Timeline|Cassette In` :!via `PlayFromStart`)
                    (:`Update`
                      (`SceneComponent.K2_SetRelativeLocationAndRotation` _tape (+ _carriagemove_2 (0.0 0.0 0.0)) (`KismetMathLibrary.MakeRotator` 0.0 _rotation 90.0) false false)
                      (bind (_direction_4 _carrigerot_2 _carriagemove_3) (`Timeline|Housing Close` :!via `ReverseFromEnd`)
                        (:`Update`
                          (`SceneComponent.K2_SetRelativeLocationAndRotation` _vcr_cassettehousing (+ _carriagemove_3 (0.0 0.0 0.0)) (`KismetMathLibrary.MakeRotator` _carrigerot_2) false false))
                        (:`Finished`
                          (set `self.HousingState` true))))))))))))))

(event `self.ReceiveActorEndOverlap`
  (params (OtherActor :type "Actor Object Reference"))
  ;[1 1 1] Trigger
  (`self.DisableInput` (`GameplayStatics.GetPlayerController` 0))
  (`Widget.RemoveFromParent` (`self.VCR_HUD`)))

(fn `UserConstructionScript`)