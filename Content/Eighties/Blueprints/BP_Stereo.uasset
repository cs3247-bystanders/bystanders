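; BP_Stereo is an interactive cassette stereo whose tape carriage opens and loads a tape when E is pressed.
; Overlapping the actor enables input and shows a HUD widget; leaving reverses both.
; Timelines animate the eject button and housing, toggle the cassette's visibility and move it once open, and close the housing after a delay started during the opening update.
; A boolean blocks retriggering until closing finishes.
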(event `self.ReceiveBeginPlay`
  ;[1 1 1] HUD
  (set `self.HousingState` true)
  (bind _returnvalue (`|CreateWidget` "/Game/Eighties/Blueprints/Blueprint_Widget.Blueprint_Widget_C"))
  (set `self.STEREO_HUD` _returnvalue))

(event `self.ReceiveActorBeginOverlap`
  (params (OtherActor :type "Actor Object Reference"))
  ;[1 1 1] Trigger
  (`self.EnableInput` (`GameplayStatics.GetPlayerController` 0))
  (`UserWidget.AddToViewport` (`self.STEREO_HUD`) 0))

(event `Key|E`
  (params (Key :type "Key Structure"))
  (bind _m_stereo_tapehousing (`self.M_Stereo_tapehousing`))
  (bind _cassette_a (`self.cassette_a`))
  ;[1 1 1] Interaction
  (:`Pressed`
    (if (`self.HousingState`)
      (set `self.HousingState` false)
      (bind (_direction _carrigerot _eject_but) (`Timeline|Open_timeline`)
        (:`Update`
          (`SceneComponent.K2_SetRelativeLocationAndRotation` :`self` (`self.M_Stereo_button_stop`) :`NewLocation` (+ _eject_but (0.0 0.0 0.0)))
          (`SceneComponent.K2_SetRelativeLocationAndRotation` _m_stereo_tapehousing (0.0 0.0 0.0) (`KismetMathLibrary.MakeRotator` _carrigerot) false false)
          (`KismetSystemLibrary.Delay` 3.0)
          (bind (_direction_2 _carrigerot_2) (`Timeline|Close_timeline` :!via `PlayFromStart`)
            (:`Update`
              (`SceneComponent.K2_SetRelativeLocationAndRotation` _m_stereo_tapehousing (0.0 0.0 0.0) (`KismetMathLibrary.MakeRotator` _carrigerot_2) false false))
            (:`Finished`
              (set `self.HousingState` true))))
        (:`Finished`
          ;[1 1 1] Load Tapehousing
          (`SceneComponent.ToggleVisibility` _cassette_a false)
          (bind (_direction_3 _rotation _tapemove) (`Timeline|Tape _IN` :!via `PlayFromStart`)
            (:`Update`
              (`SceneComponent.K2_SetRelativeLocationAndRotation` _cassette_a (+ _tapemove (0.0 0.0 0.0)) (`KismetMathLibrary.MakeRotator` 0.0 _rotation 90.0) false false))))))))

(event `self.ReceiveActorEndOverlap`
  (params (OtherActor :type "Actor Object Reference"))
  ;[1 1 1] Trigger
  (`self.DisableInput` (`GameplayStatics.GetPlayerController` 0))
  (`Widget.RemoveFromParent` (`self.STEREO_HUD`)))

(fn `UserConstructionScript`)