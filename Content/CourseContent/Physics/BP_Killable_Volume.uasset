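; A kill volume that restarts or changes the level when the player enters it and destroys any other actor that touches it.
; On player overlap with the Box, it plays an alert sound, fades the camera and audio out, then opens the level named by LevelName after a short delay.
; Other actors trigger a drum sound and fire-dust particles at the volume's location before being destroyed.
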(event `self.Box.OnComponentBeginOverlap`
  (params (OverlappedComponent :type "PrimitiveComponent Object Reference") (OtherActor :type "Actor Object Reference") (OtherComp :type "PrimitiveComponent Object Reference") (OtherBodyIndex :type Integer) (bFromSweep :type Boolean) (SweepResult :type "HitResult Structure (by ref)"))
  (bind _returnvalue (`self.K2_GetActorLocation`))
  (if (== OtherActor (`GameplayStatics.GetPlayerCharacter` 0))
    (`GameplayStatics.PlaySoundAtLocation` "/Game/Audio/SoundWaves/Effect/SW_Alert.SW_Alert" (`self.K2_GetActorLocation`))
    (`PlayerCameraManager.StartCameraFade` :`self` (`GameplayStatics.GetPlayerCameraManager` 0) :`ToAlpha` 1.0 :`Duration` 1.0 :`bShouldFadeAudio` true :`bHoldWhenFinished` true)
    (`KismetSystemLibrary.Delay` 1.0)
    (`GameplayStatics.OpenLevel` (`self.Level Name`))
    (else
      (`GameplayStatics.PlaySoundAtLocation` "/Game/Audio/SC_Drum_ElectroKick.SC_Drum_ElectroKick" _returnvalue)
      (`GameplayStatics.SpawnEmitterAtLocation` "/Game/Effects/Particles/Dust/P__Fire_Dust.P__Fire_Dust" _returnvalue)
      (`self.K2_DestroyActor` OtherActor))))

(fn `UserConstructionScript`)