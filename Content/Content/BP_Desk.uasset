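; Desk Blueprint with left and right drawers that slide open and closed along their local Y axis.
; Tick nudges a drawer by a fixed step per frame, tracking its offset between two limits, with direction chosen by that drawer's closed flag.
; The right drawer moves only while the left moving flag is false.
; Nothing in this graph sets or clears the moving and closed flags.
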(event `self.ReceiveTick`
  (params (DeltaSeconds :type "Float (single-precision)"))
  (bind _leftdrawer (`self.LeftDrawer`))
  (bind _leftoffset (`self.LeftOffset`))
  (bind _rightoffset (`self.RightOffset`))
  (bind _rightdrawer (`self.RightDrawer`))
  ;[1 1 1] Opening / Closing Tick Event
  (if (`self.isLeftMoving`)
    (if (`self.isLeftClosed`)
      (if (< _leftoffset 60.0)
        (`SceneComponent.K2_AddLocalOffset` _leftdrawer (0.0 5.0 0.0) false false)
        (set `self.LeftOffset` (+ _leftoffset 5.0)))
      (elif (> _leftoffset 0.0)
        (`SceneComponent.K2_AddLocalOffset` _leftdrawer (0.0 -5.0 0.0) false false)
        (set `self.LeftOffset` (- _leftoffset 5.0))))
    (elif (`self.isRightMoving`)
      (if (`self.isRightClosed`)
        (if (< _rightoffset 60.0)
          (`SceneComponent.K2_AddLocalOffset` _rightdrawer (0.0 5.0 0.0) false false)
          (set `self.RightOffset` (+ _rightoffset 5.0)))
        (elif (> _rightoffset 0.0)
          (`SceneComponent.K2_AddLocalOffset` _rightdrawer (0.0 -5.0 0.0) false false)
          (set `self.RightOffset` (- _rightoffset 5.0)))))))

(fn `UserConstructionScript`)