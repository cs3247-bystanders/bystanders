(event `/Game/VRIntegrator/Blueprints/I_Grabbable.Grab`
  (params (AttachTo :type "SceneComponent Object Reference") (SocketName :type Name) (Hand :type "EControllerHand Enum" :default "Left"))
  ;[1 1 1] Open Door
  (if (`self.canGoOut`)
    (`GameplayStatics.PlaySoundAtLocation` "/Game/BystanderContent/Audio/I_want_to_make_a_decision_now__I_m_teleporting_to_the_crime_scene.I_want_to_make_a_decision_now__I_m_teleporting_to_the_crime_scene")
    (`KismetSystemLibrary.Delay` 5.0)
    (`PlayerCameraManager.StartCameraFade` :`self` (`GameplayStatics.GetPlayerCameraManager` 0) :`ToAlpha` 1.0 :`Duration` 4.0)
    (`KismetSystemLibrary.Delay` 3.8)
    (`GameplayStatics.OpenLevel` (`self.LevelName`))
    (else
      (set `self.isReadyforGrab` false)
      (`GameplayStatics.PlaySoundAtLocation` "/Game/BystanderContent/Audio/Are_you_sure_you_want_to_leave.Are_you_sure_you_want_to_leave")
      (`KismetSystemLibrary.Delay` 3.5)
      (set `self.isReadyforGrab` true)
      (set `self.canGoOut` true))))

(fn `BeginFocus`
  (`PrimitiveComponent.SetRenderCustomDepth` (`self.Mesh_Door_02`) true))

(fn `CanBeGrabbed`
  (returns (IsGrabbableReady :type Boolean))
  (return (`self.isReadyforGrab`)))

(fn `EndFocus`
  (`PrimitiveComponent.SetRenderCustomDepth` (`self.Mesh_Door_02`) false))

(fn `UserConstructionScript`)