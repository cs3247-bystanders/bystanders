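; BP_Door_04 is a grabbable door that takes the player to another level.
; Gaining or losing focus toggles custom depth rendering on its MeshDoor02 mesh, and the IsReadyforGrab flag decides whether it can be grabbed.
; Grabbing it starts a held camera fade-out, then opens the level named in LevelName just before the fade completes.
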(event `self.ReceiveBeginPlay`
  ;[1 1 1] Open Door
)

(event `/Game/VRIntegrator/Blueprints/I_Grabbable.Grab`
  (params (AttachTo :type "SceneComponent Object Reference") (SocketName :type Name) (Hand :type "EControllerHand Enum" :default "Left"))
  ;[1 1 1] Open Door
  (`PlayerCameraManager.StartCameraFade` :`self` (`GameplayStatics.GetPlayerCameraManager` 0) :`ToAlpha` 1.0 :`Duration` 4.0 :`bHoldWhenFinished` true)
  (`KismetSystemLibrary.Delay` 3.8)
  (`GameplayStatics.OpenLevel` (`self.LevelName`)))

(fn `BeginFocus`
  (`PrimitiveComponent.SetRenderCustomDepth` (`self.Mesh_Door_02`) true))

(fn `CanBeGrabbed`
  (returns (IsGrabbableReady :type Boolean))
  (return (`self.isReadyforGrab`)))

(fn `EndFocus`
  (`PrimitiveComponent.SetRenderCustomDepth` (`self.Mesh_Door_02`) false))

(fn `UserConstructionScript`)