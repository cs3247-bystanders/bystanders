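; Lockable desk door that the player can grab to swing open and closed, playing a rejection sound while locked.
; Overlapping KeyHole with a key Blueprint unlocks it, hides the key and destroys the lock components.
; Grab flip-flops a yaw Timeline forward and back, with cross-resetting DoOnce nodes gating the sounds.
; OnFocus shows a widget and optional custom-depth outline, cleared by a retriggerable delay when focus calls stop.
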(event `/Game/VRIntegrator/Blueprints/I_Grabbable.Grab`
  (params (AttachTo :type "SceneComponent Object Reference") (SocketName :type Name) (Hand :type "EControllerHand Enum" :default "Left"))
  ;[1 1 1] Open Door
  (if (`self.isUnlocked`)
    (`/Engine/EditorBlueprintResources/StandardMacros.FlipFlop`
      (:`A`
        (`|ExecutionSequence`
          (:`then_0`
            (`/Engine/EditorBlueprintResources/StandardMacros.DoOnce` false :!label _label
              (:`Completed`
                (`GameplayStatics.PlaySoundAtLocation` "/Game/VHCabinet/Audio/Cues/Cue_OpenDoor_02.Cue_OpenDoor_02")
                (goto _label_3 :!via `Reset`))))
          (:`then_1`
            (bind (_direction _doorrotater) (`Timeline|Door` :!label _label_2)
              (:`Update`
                (`SceneComponent.K2_SetRelativeRotation` (`self.Mesh_Desk_Door_01_02`) (`KismetMathLibrary.MakeRotator` 0.0 0.0 _doorrotater) false false))))))
      (:`B`
        (`|ExecutionSequence`
          (:`then_0`
            (goto _label_2 :!via `Reverse`))
          (:`then_1`
            (`/Engine/EditorBlueprintResources/StandardMacros.DoOnce` false :!label _label_3
              (:`Completed`
                (`GameplayStatics.PlaySoundAtLocation` "/Game/VHCabinet/Audio/Wavs/S_CloseDoor_02.S_CloseDoor_02")
                (goto _label :!via `Reset`)))))))
    (else
      (`GameplayStatics.PlaySoundAtLocation` "/Game/VHCabinet/Audio/Cues/Cue_PushButton.Cue_PushButton"))))

(event `/Game/VHCabinet/Blueprints/BP_InteractInterface.On Focus`
  ;[1 1 1] Outline
  (`|ExecutionSequence`
    (:`then_0`
      (if (`self.Outline on/off`)
        (`self.BeginFocus`))
      (set `self.TimeOutlineEnd` 0.1)
      (`KismetSystemLibrary.RetriggerableDelay` (`self.TimeOutlineEnd`))
      (`self.EndFocus`)
      (`Widget.RemoveFromParent` (stale _returnvalue))
      (`self.Reset` false))
    (:`then_1`
      (`/Engine/EditorBlueprintResources/StandardMacros.Do N` 1 :!label _label_4
        (:`Exit`
          (bind _returnvalue (`|CreateWidget` "/Game/VHCabinet/UMG/Door_Widget.Door_Widget_C"))
          (`UserWidget.AddToViewport` _returnvalue 0))))))

(event `Reset`
  (params (NewParam :type Boolean))
  ;[1 1 1] Outline
  (goto _label_4 :!via `Reset`))

(event `self.KeyHole.OnComponentBeginOverlap`
  (params (OverlappedComponent :type "PrimitiveComponent Object Reference") (OtherActor :type "Actor Object Reference") (OtherComp :type "PrimitiveComponent Object Reference") (OtherBodyIndex :type Integer) (bFromSweep :type Boolean) (SweepResult :type "HitResult Structure (by ref)"))
  (bind _asmesh_key_blueprint (cast `/Game/BystanderContent/Scene1BPPickUpObjects/Mesh_Key_Blueprint` OtherActor))
  (set `self.isUnlocked` true)
  (`self.K2_SetActorLocation` _asmesh_key_blueprint (0.0 0.0 0.0) false false)
  (`SceneComponent.SetVisibility` (`StaticMeshActor.StaticMeshComponent` _asmesh_key_blueprint) false false)
  (`GameplayStatics.PlaySoundAtLocation` "/Game/VHCabinet/Audio/Cues/Cue_Light.Cue_Light")
  (`ActorComponent.K2_DestroyComponent` (`self.Lock_Part`))
  (`ActorComponent.K2_DestroyComponent` (`self.Lock`)))

(fn `BeginFocus`
  (`PrimitiveComponent.SetRenderCustomDepth` (`self.Mesh_Desk_Door_01_02`) true))

(fn `CanBeGrabbed`
  (returns (IsGrabbableReady :type Boolean))
  (return true))

(fn `EndFocus`
  (`PrimitiveComponent.SetRenderCustomDepth` (`self.Mesh_Desk_Door_01_02`) false))

(fn `UserConstructionScript`)