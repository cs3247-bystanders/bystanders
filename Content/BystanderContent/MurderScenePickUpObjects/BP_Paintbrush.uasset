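; BP_Paintbrush is a grabbable paintbrush prop, filed among the murder scene pick-up objects, with a configurable paint material applied in the construction script.
; Grab turns off physics, attaches the actor to the given parent and socket keeping its world transform, and clears the outline; Release detaches it and restores physics.
; The outline uses custom depth and stencil.
; CanBeGrabbed always returns true, ignoring the IsReadyForGrab flag set by SetGrabbaleEnabled.
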(event `/Game/VRIntegrator/Blueprints/I_Grabbable.Grab`
  (params (AttachTo :type "SceneComponent Object Reference") (SocketName :type Name) (Hand :type "EControllerHand Enum" :default "Left"))
  ;[1 1 1] Grab/Release Interaction
  (`PrimitiveComponent.SetSimulatePhysics` (`self.StaticMeshComponent`) false)
  (`SceneComponent.K2_AttachToComponent` (`self.RootComponent`) AttachTo SocketName "KeepWorld" "KeepWorld" "KeepWorld" true)
  (`/Game/VRIntegrator/Blueprints/I_Grabbable.SetOutline` false))

(event `/Game/VRIntegrator/Blueprints/I_Grabbable.Release`
  ;[1 1 1] Grab/Release Interaction
  (`PrimitiveComponent.SetSimulatePhysics` (`self.StaticMeshComponent`) true)
  (`self.K2_DetachFromActor` "KeepWorld" "KeepWorld" "KeepWorld"))

(event `/Game/VRIntegrator/Blueprints/I_Grabbable.SetOutline`
  (params (InEnable :type Boolean) (InStencil :type Integer))
  (bind _staticmeshcomponent (`self.StaticMeshComponent`))
  ;[1 1 1] Grab/Release Interaction
  (`PrimitiveComponent.SetCustomDepthStencilValue` _staticmeshcomponent InStencil)
  (`PrimitiveComponent.SetRenderCustomDepth` _staticmeshcomponent InEnable))

(event `/Game/VRIntegrator/Blueprints/I_Grabbable.SetGrabbaleEnabled`
  (params (Enabled :type Boolean))
  ;[1 1 1] Grab/Release Interaction
  (set `self.IsReadyForGrab` Enabled))

(fn `CanBeGrabbed`
  (returns (IsGrabbableReady :type Boolean))
  (return true))

(fn `UserConstructionScript`
  (`PrimitiveComponent.SetMaterial` (`self.StaticMeshComponent`) 0 (`self.paintMaterial`)))