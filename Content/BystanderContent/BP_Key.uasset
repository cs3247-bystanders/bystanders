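; BP_Key is a key that gets physically pulled toward a magnet while in range.
; Overlap on its sphere collision stores any I_Magnet actor and enables attraction, while end overlap disables it only for BP_Magnet.
; Each Tick while attracted, the key mesh receives an acceleration-based force toward the magnet's mesh, scaled by MagnetSpeed.
; The construction script sizes the collision sphere from the key mesh's local Y extent.
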(event `self.ReceiveTick`
  (params (DeltaSeconds :type "Float (single-precision)"))
  (set `self.deltaSeconds` DeltaSeconds)
  (if (`self.isAttracted`)
    (bind _mesh (`/Game/BystanderContent/I_Magnet.GetMesh` (`self.magnet`)))
    (`PrimitiveComponent.AddForce` (`self.KeyMesh`) (* (`KismetMathLibrary.GetDirectionUnitVector` (`SceneComponent.K2_GetComponentLocation` (`self.KeyMesh`)) (`SceneComponent.K2_GetComponentLocation` _mesh)) (`self.magnetSpeed`)) "None" true)))

(event `self.KeyCollision.OnComponentBeginOverlap`
  (params (OverlappedComponent :type "PrimitiveComponent Object Reference") (OtherActor :type "Actor Object Reference") (OtherComp :type "PrimitiveComponent Object Reference") (OtherBodyIndex :type Integer) (bFromSweep :type Boolean) (SweepResult :type "HitResult Structure (by ref)"))
  (bind _asi_magnet (cast `/Game/BystanderContent/I_Magnet` OtherActor))
  (set `self.isAttracted` true)
  (set `self.magnet` _asi_magnet))

(event `self.KeyCollision.OnComponentEndOverlap`
  (params (OverlappedComponent :type "PrimitiveComponent Object Reference") (OtherActor :type "Actor Object Reference") (OtherComp :type "PrimitiveComponent Object Reference") (OtherBodyIndex :type Integer))
  (cast `/Game/BystanderContent/BP_Magnet` OtherActor)
  (set `self.isAttracted` false))

(fn `UserConstructionScript`
  (bind (_min _max) (`StaticMeshComponent.GetLocalBounds` (`self.KeyMesh`)))
  (`SphereComponent.SetSphereRadius` (`self.KeyCollision`) (/ (- (.y _max) (.y _min)) 1.75) true))