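; BP_TV_Knob is a grabbable TV knob that controls the volume of a sound source.
; Each tick it maps the knob mesh's world pitch through a sine curve, scaled by MaxVolume, onto the sound source's audio component volume multiplier.
; CanBeGrabbed reports the IsReadyForGrab flag.
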(event `self.ReceiveTick`
  (params (DeltaSeconds :type "Float (single-precision)"))
  (`AudioComponent.SetVolumeMultiplier` (`AmbientSound.AudioComponent` (`self.Sound Source`)) (* (+ (`KismetMathLibrary.DegSin` (- (.pitch (`SceneComponent.K2_GetComponentRotation` (`self.KnobMesh`))) 90.0)) 1.0) (`self.maxVolume`))))

(fn `CanBeGrabbed`
  (returns (IsGrabbableReady :type Boolean))
  (return (`self.isReadyForGrab`)))

(fn `UserConstructionScript`)