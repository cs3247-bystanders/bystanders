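; BP_TV_Switch is an interactable wall-style switch that flips on or off and reports its state to a linked TV.
; Grab or primary interact toggles it and each switch in its dependent list, without cascading further, suggesting a linked-switch puzzle.
; Toggling rotates the switch through timelines, then swaps the bulb material and sends a positive or negative step to the TV.
; The construction script matches rotation and bulb to the initial state.
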(event `/Game/VRIntegrator/Blueprints/I_Grabbable.Grab`
  (params (AttachTo :type "SceneComponent Object Reference") (SocketName :type Name) (Hand :type "EControllerHand Enum" :default "Left"))
  (`self.Toggle`)
  (for _array_element (`self.depdentSwitches`)
    (`self.Toggle` _array_element)))

(event `Toggle`
  (bind _output_get (set `self.isOn` (not (`self.isOn`))))
  (if _output_get
    (bind (_direction _doorrotater) (`Timeline|Timeline_0` :!via `PlayFromStart`)
      (:`Update`
        (`SceneComponent.K2_SetRelativeRotation` (`self.Switch`) (`KismetMathLibrary.MakeRotator` _doorrotater) false false))
      (:`Finished`
        (`PrimitiveComponent.SetMaterial` (`self.SM_LightBulb2`) 1 "/Game/Radio/Materials/MI_Emission.MI_Emission")
        (`/Game/Eighties/Blueprints/BP_TV.Update Switch` (`self.tv`) 2)))
    (else
      (bind (_direction_2 _doorrotater_2) (`Timeline|Timeline_1` :!via `ReverseFromEnd`)
        (:`Update`
          (`SceneComponent.K2_SetRelativeRotation` (`self.Switch`) (`KismetMathLibrary.MakeRotator` _doorrotater_2) false false))
        (:`Finished`
          (`PrimitiveComponent.SetMaterial` (`self.SM_LightBulb2`) 1 "/Game/Survival_Items_Pack/Materials/Environment/M_Black.M_Black")
          (`/Game/Eighties/Blueprints/BP_TV.Update Switch` (`self.tv`) -2))))))

(fn `CanBeGrabbed`
  (returns (IsGrabbableReady :type Boolean))
  (return false))

(fn `GetInteractions()`
  (returns (InteractionTexts :type "Array of String"))
  (return))

(fn `PriInteract()`
  (returns (Success :type Boolean))
  (`self.Toggle`)
  (for _array_element (`self.depdentSwitches`)
    (`self.Toggle` _array_element))
  (return true))

(fn `SecInteract()`
  (returns (Success :type Boolean))
  (return false))

(fn `UserConstructionScript`
  (if (`self.isOn`)
    (`SceneComponent.K2_SetRelativeRotation` (`self.Switch`) (struct :`Roll` 40.0) false false)
    (`PrimitiveComponent.SetMaterial` (`self.SM_LightBulb2`) 1 "/Game/Radio/Materials/MI_Emission.MI_Emission")
    (else
      (`SceneComponent.K2_SetRelativeRotation` (`self.Switch`) (struct :`Roll` -40.0) false false)
      (`PrimitiveComponent.SetMaterial` (`self.SM_LightBulb2`) 1 "/Game/Survival_Items_Pack/Materials/Environment/M_Black.M_Black"))))