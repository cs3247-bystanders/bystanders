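; BP_Lever is a grabbable lever that flips between two positions and triggers a car to turn.
; Grab and primary interaction both call Toggle, where a FlipFlop alternates playing a timeline forward or in reverse to roll the static mesh.
; When the timeline finishes, it calls Turn on the referenced Car.
; Secondary interaction does nothing.
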(event `/Game/VRIntegrator/Blueprints/I_Grabbable.Grab`
  (params (AttachTo :type "SceneComponent Object Reference") (SocketName :type Name) (Hand :type "EControllerHand Enum" :default "Left"))
  (`self.Toggle`))

(event `Toggle`
  (`/Engine/EditorBlueprintResources/StandardMacros.FlipFlop`
    (:`A`
      (bind (_direction _doorrotater) (`Timeline|Timeline_0` :!via `PlayFromStart` :!label _label)
        (:`Update`
          (`SceneComponent.K2_SetRelativeRotation` (`self.StaticMesh`) (`KismetMathLibrary.MakeRotator` _doorrotater) false false))
        (:`Finished`
          (`/Game/BystanderContent/BP_Car.Turn` (`self.car`)))))
    (:`B`
      (goto _label :!via `ReverseFromEnd`))))

(fn `CanBeGrabbed`
  (returns (IsGrabbableReady :type Boolean))
  (return true))

(fn `GetInteractions()`
  (returns (InteractionTexts :type "Array of String"))
  (return))

(fn `PriInteract()`
  (returns (Success :type Boolean))
  (`self.Toggle`)
  (return true))

(fn `SecInteract()`
  (returns (Success :type Boolean))
  (return false))

(fn `UserConstructionScript`)