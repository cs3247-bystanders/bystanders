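; Level manager Blueprint that tracks whether a set of element properties matches expected values and decides the level's success or failure.
; ChangeAlignment finds the matching property in IsElementsAligned, marks it correct if the passed value equals the stored one, and debug-prints the array.
; EvaluateElementsAlignment requires every entry to be correct, then fades the camera out and opens FinishLevel or FailLevel.
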(event `EvaluateElementsAlignment`
  (bind _returnvalue (`GameplayStatics.GetPlayerCameraManager` 0))
  (for _array_element (`self.isElementsAligned`)
    (if (== (`.isCorrect_15_D806E8F24198EA2F1A50778BFFEAFB2F` (break `/Game/BystanderContent/ConfigurationPair` _array_element)) true)
      (set `self.isLevelSuccess` true)
      (else
        (set `self.isLevelSuccess` false)
        (break))))
  (if (`self.isLevelSuccess`)
    (`PlayerCameraManager.StartCameraFade` :`self` _returnvalue :`ToAlpha` 1.0 :`Duration` 4.0)
    (`KismetSystemLibrary.Delay` 3.8)
    (`GameplayStatics.OpenLevel` "FinishLevel")
    (else
      (`PlayerCameraManager.StartCameraFade` :`self` _returnvalue :`ToAlpha` 1.0 :`Duration` 4.0)
      (`KismetSystemLibrary.Delay` 3.8)
      (`GameplayStatics.OpenLevel` "FailLevel"))))

(fn `ChangeAlignment`
  (params (property :type String) (value :type String))
  (bind _iselementsaligned (`self.isElementsAligned`))
  (for (_array_element _array_index) _iselementsaligned
    (bind (_properties _value) (break `/Game/BystanderContent/ConfigurationPair` _array_element))
    (if (`KismetStringLibrary.EqualEqual_StrStr` _properties property)
      (`KismetArrayLibrary.Array_Set` _iselementsaligned _array_index (make `/Game/BystanderContent/ConfigurationPair` _properties _value (`KismetStringLibrary.EqualEqual_StrStr` _value value)))
      (for _array_element_2 (`self.isElementsAligned`)
        (bind (_properties_2 _value_2 _iscorrect) (break `/Game/BystanderContent/ConfigurationPair` _array_element_2))
        (`KismetSystemLibrary.PrintString` (`KismetStringLibrary.Concat_StrStr` _properties_2 _value_2 (`KismetStringLibrary.Conv_BoolToString` _iscorrect))))
      (return))))

(fn `UserConstructionScript`)