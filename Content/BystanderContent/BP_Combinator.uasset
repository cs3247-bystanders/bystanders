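; BP_Combinator is a crafting manager that turns two registered ingredient actors into a recipe result.
; RegisterAsIngredient fills the First and Second slots, and Tick runs CombineIngredients once both are set.
; Order-independent recipe matching uses I_Combinable indices, then spawns the result at First's transform, plays a thud and destroys both ingredients.
; Tick clears the slots instead when DeltaSeconds modulo five is zero, testing frame delta rather than elapsed time.
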(event `self.ReceiveTick`
  (params (DeltaSeconds :type "Float (single-precision)"))
  (if (== (mod DeltaSeconds 5.0) 0.0)
    (`self.FreeUpIngredients`)
    (elif (!= (`self.first`) null)
      (if (!= (`self.second`) null)
        (`self.CombineIngredients`)))))

(fn `CombineIngredients`
  (for _array_element (`self.recipes`)
    (bind _asi_combinable (cast `/Game/BystanderContent/I_Combinable` (`self.first`)))
    (bind _index (`/Game/BystanderContent/I_Combinable.GetIngredientIndex` _asi_combinable))
    (bind _asi_combinable_2 (cast `/Game/BystanderContent/I_Combinable` (`self.second`)))
    (bind _index_2 (`/Game/BystanderContent/I_Combinable.GetIngredientIndex` _asi_combinable_2))
    (bind (_first _second _result) (break `/Game/BystanderContent/RecipePair` _array_element))
    (if (or (and (== _index _first) (== _index_2 _second)) (and (== _index _second) (== _index_2 _first)))
      (bind _returnvalue (`|SpawnActorFromClass` _result (`self.GetTransform` (`self.first`)) "Undefined" "OverrideRootScale" null null))
      (`GameplayStatics.PlaySoundAtLocation` "/Game/CourseContent/Audio/SoundWaves/Effect/SW_Thud_1.SW_Thud_1" (`self.K2_GetActorLocation` _returnvalue))
      (`self.K2_DestroyActor` (`self.first`))
      (`self.K2_DestroyActor` (`self.second`))
      (break)))
  (return))

(fn `FreeUpIngredients`
  (set `self.first` null)
  (set `self.second` null)
  (return))

(fn `RegisterAsIngredient`
  (params (candidate :type "Actor Object Reference"))
  (if (== (`self.first`) null)
    (set `self.first` null)
    (set `self.first` candidate)
    (elif (== (`self.second`) null)
      (set `self.second` candidate)))
  (return))

(fn `UserConstructionScript`)