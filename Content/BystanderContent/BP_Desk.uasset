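; BP_Desk is an interactable desk with left and right drawers that slide open and closed.
; Primary interact toggles the left drawer and secondary the right, updating prompt texts returned by GetInteractions; a locked right drawer tells the player a key is needed.
; Tick slides the flagged drawer in fixed per-frame steps until its offset reaches a limit, so speed depends on frame rate and left motion takes priority.
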(event `self.ReceiveTick`
  (params (DeltaSeconds :type "Float (single-precision)"))
  (bind _leftdrawer (`self.LeftDrawer`))
  (bind _leftoffset (`self.LeftOffset`))
  (bind _rightoffset (`self.RightOffset`))
  (bind _rightdrawer (`self.RightDrawer`))
  ;[1 1 1] Opening / Closing Tick Event
  (if (`self.isLeftMoving`)
    (if (`self.isLeftClosed`)
      (if (< _leftoffset 60.0)
        (`SceneComponent.K2_AddLocalOffset` _leftdrawer (0.0 5.0 0.0) false false)
        (set `self.LeftOffset` (+ _leftoffset 5.0))
        (else
          (set `self.isLeftMoving` false)))
      (elif (> _leftoffset 0.0)
        (`SceneComponent.K2_AddLocalOffset` _leftdrawer (0.0 -5.0 0.0) false false)
        (set `self.LeftOffset` (- _leftoffset 5.0))
        (else
          (set `self.isLeftMoving` false))))
    (elif (`self.isRightMoving`)
      (if (`self.isRightClosed`)
        (if (< _rightoffset 60.0)
          (`SceneComponent.K2_AddLocalOffset` _rightdrawer (0.0 5.0 0.0) false false)
          (set `self.RightOffset` (+ _rightoffset 5.0))
          (else
            (set `self.isRightMoving` false)))
        (elif (> _rightoffset 0.0)
          (`SceneComponent.K2_AddLocalOffset` _rightdrawer (0.0 -5.0 0.0) false false)
          (set `self.RightOffset` (- _rightoffset 5.0))
          (else
            (set `self.isRightMoving` false)))))))

(fn `GetInteractions()`
  (returns (InteractionTexts :type "Array of String"))
  (return (`self.interactionTexts`)))

(fn `PriInteract()`
  (returns (Success :type Boolean))
  (bind _isleftmoving (`self.isLeftMoving`))
  (bind _interactiontexts (`self.interactionTexts`))
  (if (`self.isLeftClosed`)
    (if (not _isleftmoving)
      (set `self.isLeftClosed` false)
      (`KismetArrayLibrary.Array_Set` _interactiontexts 0 "Close Left")
      (set `self.isLeftMoving` true)
      (return false))
    (elif (not _isleftmoving)
      (set `self.isLeftClosed` true)
      (`KismetArrayLibrary.Array_Set` _interactiontexts 0 "Open Left")
      (set `self.isLeftMoving` true)
      (return false))))

(fn `SecInteract()`
  (returns (Success :type Boolean))
  (bind _interactiontexts (`self.interactionTexts`))
  (bind _isrightmoving (`self.isRightMoving`))
  (if (`self.isRightLocked`)
    (bind _asbp_bystander_player (cast `/Game/BystanderContent/BP_Bystander_Player` (`GameplayStatics.GetPlayerCharacter` 0)))
    (`/Game/BystanderContent/BP_Bystander_Player.ChangePromptText` _asbp_bystander_player "It's locked. I will need a key")
    (elif (`self.isRightClosed`)
      (if (not _isrightmoving)
        (set `self.isRightClosed` false)
        (`KismetArrayLibrary.Array_Set` _interactiontexts 1 "Close Right")
        (set `self.isRightMoving` true)
        (return false))
      (elif (not _isrightmoving)
        (set `self.isRightClosed` true)
        (`KismetArrayLibrary.Array_Set` _interactiontexts 1 "Open Right")
        (set `self.isRightMoving` true)
        (return false)))))

(fn `UserConstructionScript`)