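; BP_Note is an interactable Scene 1 note that the player rolls and unrolls to show or hide a message.
; Primary interaction yaws two cube pieces 180 degrees, sets a dynamic material's "appear" parameter to 1, then calls makeTextVisible.
; That event toggles ReturnMapMessage and switches the prompt returned by GetInteractions between "Roll Up" and "Unroll".
; Secondary interaction does nothing, and both interactions return false.
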(event `makeTextVisible`
  (bind _interactiontexts (`self.interactionTexts`))
  (bind _returnmapmessage (`self.ReturnMapMessage`))
  (`SceneComponent.ToggleVisibility` _returnmapmessage false)
  (if (`SceneComponent.bVisible` _returnmapmessage)
    (`KismetArrayLibrary.Array_Set` _interactiontexts 0 "Roll Up")
    (else
      (`KismetArrayLibrary.Array_Set` _interactiontexts 0 "Unroll"))))

(fn `GetInteractions()`
  (returns (InteractionTexts :type "Array of String"))
  (return (`self.interactionTexts`)))

(fn `PriInteract()`
  (returns (Success :type Boolean))
  ;[1 1 1] Expand the note to twice the size
  (`SceneComponent.K2_AddLocalRotation` (`self.Cube1`) (`KismetMathLibrary.MakeRotator` 0.0 0.0 180.0) false false)
  (`SceneComponent.K2_AddLocalRotation` (`self.Cube2`) (`KismetMathLibrary.MakeRotator` 0.0 0.0 180.0) false false)
  (bind _returnvalue (`PrimitiveComponent.CreateDynamicMaterialInstance` (`self.Cubes`) 0 null))
  (`MaterialInstanceDynamic.SetScalarParameterValue` _returnvalue "appear" 1.0)
  (`self.makeTextVisible`)
  (return false))

(fn `SecInteract()`
  (returns (Success :type Boolean))
  (return false))

(fn `UserConstructionScript`)