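; BP_Map is an interactable map prop that unrolls once, faked by crossfading from a cylinder mesh to a plane mesh.
; Primary interaction calls Unroll behind an IsDone flag, while secondary interaction returns false.
; Unroll drives fade parameters on dynamic material instances with two timelines, fading the cylinder out and, after a delay triggered from the first timeline's update, fading the plane in.
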(event `Unroll`
  ;[1 1 1] Fade from cylinder map to plane map
  (bind _returnvalue (`PrimitiveComponent.CreateDynamicMaterialInstance` (`self.Cylinder`) 0 "/Game/BystanderContent/Scene1Objects/M_MapMaterial.M_MapMaterial"))
  (bind (_direction _newtrack_0) (`Timeline|fadeTime` :!via `PlayFromStart`)
    (:`Update`
      (`MaterialInstanceDynamic.SetScalarParameterValue` _returnvalue "fadeOut" _newtrack_0)
      (`KismetSystemLibrary.Delay` 1.6)
      (bind _returnvalue_2 (`PrimitiveComponent.CreateDynamicMaterialInstance` (`self.Plane`) 0 "/Game/BystanderContent/Scene1Objects/M_MapMaterial_Fadein.M_MapMaterial_FadeIn"))
      (bind (_direction_2 _newtrack_0_2) (`Timeline|Timeline_0` :!via `PlayFromStart`)
        (:`Update`
          (`MaterialInstanceDynamic.SetScalarParameterValue` _returnvalue_2 "fadeIn" _newtrack_0_2))))))

(fn `GetInteractions()`
  (returns (InteractionTexts :type "Array of String"))
  (return))

(fn `PriInteract()`
  (returns (Success :type Boolean))
  (if (not (`self.isDone`))
    (`self.Unroll`)
    (set `self.isDone` true)
    (return false)))

(fn `SecInteract()`
  (returns (Success :type Boolean))
  (return false))

(fn `UserConstructionScript`)