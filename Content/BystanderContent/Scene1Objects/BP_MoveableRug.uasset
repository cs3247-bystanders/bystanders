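; BP_MoveableRug is a Scene 1 rug object that flips up or down when interacted with.
; The primary interaction toggles an IsFlipped flag, instantly rotating the Rug component 25 degrees on its local roll axis and printing the new state on screen.
; The secondary interaction and interaction query are empty stubs, and an unused time-based sine expression remains in the primary interaction graph.
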(event `self.ReceiveTick`
  (params (DeltaSeconds :type "Float (single-precision)")))

(fn `GetInteractions()`
  (returns (InteractionTexts :type "Array of String"))
  (return))

(fn `PriInteract()`
  (returns (Success :type Boolean))
  (if (`self.isFlipped`)
    (`SceneComponent.K2_AddLocalRotation` (`self.Rug`) (`KismetMathLibrary.MakeRotator` -25.0) false false)
    (`KismetSystemLibrary.PrintString` "Rug is flipped down!")
    (set `self.isFlipped` false)
    (else
      (`SceneComponent.K2_AddLocalRotation` (`self.Rug`) (`KismetMathLibrary.MakeRotator` 25.0) false false)
      (`KismetSystemLibrary.PrintString` "Rug is flipped up!")
      (set `self.isFlipped` true)))
  (return false))

(fn `SecInteract()`
  (returns (Success :type Boolean))
  (return false))

(fn `UserConstructionScript`)