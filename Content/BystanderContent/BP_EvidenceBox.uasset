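; BP_EvidenceBox is an evidence box that tracks which weapons are placed inside it and reports whether the correct one is present.
; Box overlap begin and end add or subtract each overlapping I_Weapon actor's GetWeaponValue to a running Sum.
; After every change, it sets LevelAdmin's "weapon" alignment to "greenKnife" when Sum equals exactly one, otherwise to "other".
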(event `CheckCorrectWeapon`
  (bind _leveladmin (`self.levelAdmin`))
  (if (== (`self.sum`) 1)
    (`/Game/BystanderContent/BP_LevelAdmin.ChangeAlignment` _leveladmin "weapon" "greenKnife")
    (else
      (`/Game/BystanderContent/BP_LevelAdmin.ChangeAlignment` _leveladmin "weapon" "other"))))

(event `self.Box.OnComponentBeginOverlap`
  (params (OverlappedComponent :type "PrimitiveComponent Object Reference") (OtherActor :type "Actor Object Reference") (OtherComp :type "PrimitiveComponent Object Reference") (OtherBodyIndex :type Integer) (bFromSweep :type Boolean) (SweepResult :type "HitResult Structure (by ref)"))
  (bind _asi_weapon (cast `/Game/BystanderContent/I_Weapon` OtherActor))
  (bind _value (`/Game/BystanderContent/I_Weapon.getWeaponValue` _asi_weapon))
  (set `self.sum` (+ (`self.sum`) _value))
  (`self.CheckCorrectWeapon` :!label _label))

(event `self.Box.OnComponentEndOverlap`
  (params (OverlappedComponent :type "PrimitiveComponent Object Reference") (OtherActor :type "Actor Object Reference") (OtherComp :type "PrimitiveComponent Object Reference") (OtherBodyIndex :type Integer))
  (bind _asi_weapon (cast `/Game/BystanderContent/I_Weapon` OtherActor))
  (bind _value (`/Game/BystanderContent/I_Weapon.getWeaponValue` _asi_weapon))
  (set `self.sum` (- (`self.sum`) _value))
  (goto _label))

(fn `UserConstructionScript`)