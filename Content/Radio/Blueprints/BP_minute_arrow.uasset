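; Grabbable minute hand, stored under the Radio assets, that the player steps forward in ten-minute increments.
; Each Grab rotates the MinutesArrow component 60 degrees locally and advances Minutes by ten, wrapping at 60.
; It then sends the new value as a string to LevelAdmin through ChangeAlignment under the "minute" property.
; CanBeGrabbed always returns true, so the hand is never locked.
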(event `/Game/VRIntegrator/Blueprints/I_Grabbable.Grab`
  (params (AttachTo :type "SceneComponent Object Reference") (SocketName :type Name) (Hand :type "EControllerHand Enum" :default "Left"))
  (`SceneComponent.K2_AddLocalRotation` (`self.MinutesArrow`) (struct :`Pitch` 60.0) false false)
  (bind _output_get (set `self.minutes` (mod (+ (`self.minutes`) 10) 60)))
  (`/Game/BystanderContent/BP_LevelAdmin.ChangeAlignment` (`self.levelAdmin`) "minute" (`KismetStringLibrary.Conv_IntToString` _output_get)))

(fn `CanBeGrabbed`
  (returns (IsGrabbableReady :type Boolean))
  (return true))

(fn `UserConstructionScript`)