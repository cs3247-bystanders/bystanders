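; Grabbable hour hand actor that lets the player set the hour, stored among the Radio assets.
; Each Grab rotates HoursArrow by a fixed one-hour step and advances Hours, wrapping on a 12-hour cycle.
; It then passes the new hour as a string to LevelAdmin.ChangeAlignment under the "hour" property.
; CanBeGrabbed always returns true, so the hand is always interactable.
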(event `/Game/VRIntegrator/Blueprints/I_Grabbable.Grab`
  (params (AttachTo :type "SceneComponent Object Reference") (SocketName :type Name) (Hand :type "EControllerHand Enum" :default "Left"))
  (`SceneComponent.K2_AddLocalRotation` (`self.HoursArrow`) (struct :`Pitch` -30.0) false false)
  (bind _output_get (set `self.hours` (mod (+ (`self.hours`) 1) 12)))
  (`/Game/BystanderContent/BP_LevelAdmin.ChangeAlignment` (`self.levelAdmin`) "hour" (`KismetStringLibrary.Conv_IntToString` _output_get)))

(fn `CanBeGrabbed`
  (returns (IsGrabbableReady :type Boolean))
  (return true))

(fn `UserConstructionScript`)