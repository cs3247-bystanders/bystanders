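; VR dockable window actor that displays a UMG widget in a mesh frame with a drag bar and close button.
; Construction creates the widget at a set resolution, while Tick rescales and positions the meshes from scale and aspect ratio.
; Hover state recolors the bar and button through dynamic materials.
; Option flags toggle each part's visibility and collision, and showing or hiding switches collision for the whole window.
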(event `self.ReceiveBeginPlay`
  (`self.Initialize`))

(event `self.ReceiveTick`
  (params (DeltaSeconds :type "Float (single-precision)"))
  (`self.UpdateWindowMeshTransforms`))

(fn `GetSize`
  (returns (OutSize :type "Vector2D Structure"))
  (locals (AspectRatio :type "Float (double-precision)"))
  (bind _scale (`self.Scale`))
  (bind (_x _y) (`KismetMathLibrary.BreakVector2D` (`self.Resolution`)))
  (set `local.AspectRatio` (/ _x _y))
  (return (`KismetMathLibrary.MakeVector2D` _scale (/ _scale (`local.AspectRatio`)))))

(fn `GetWorldScaleFactor`
  (returns (WorldScaleFactor :type "Float (double-precision)"))
  (return (/ (`HeadMountedDisplayFunctionLibrary.GetWorldToMetersScale`) 100.0)))

(fn `Initialize`
  (`|ExecutionSequence`
    (:`then_0`
      (bind _returnvalue (`PrimitiveComponent.CreateDynamicMaterialInstance` (`self.SelectionMesh`) 0 "/Game/VRIntegrator/Materials/MI_WindowGizmo.MI_WindowGizmo"))
      (set `self.MIDSelectionBar` _returnvalue)
      (bind _returnvalue_2 (`PrimitiveComponent.CreateDynamicMaterialInstance` (`self.SelectionMesh`) 1 "/Game/VRIntegrator/Materials/MI_TranslucentWindowGizmo.MI_TranslucentWindowGizmo"))
      (set `self.MIDSelectionBarTranslucent` _returnvalue_2))
    (:`then_1`
      (bind _returnvalue_3 (`PrimitiveComponent.CreateDynamicMaterialInstance` (`self.CloseMesh`) 0 "/Game/VRIntegrator/Materials/MI_WindowGizmo.MI_WindowGizmo"))
      (set `self.MIDCloseButton` _returnvalue_3)
      (bind _returnvalue_4 (`PrimitiveComponent.CreateDynamicMaterialInstance` (`self.CloseMesh`) 1 "/Game/VRIntegrator/Materials/MI_TranslucentWindowGizmo.MI_TranslucentWindowGizmo"))
      (set `self.MIDCloseButtonTranslucent` _returnvalue_4))
    (:`then_2`
      (`self.UpdateHoverState`)
      (`ActorComponent.SetTickableWhenPaused` (`self.WidgetDisplayed`) true))
    (:`then_3`
      (if (`self.IsLevelPlaced`)
        (`self.ShowDockableWindow` (`self.IsVisibleOnMapLoad`) true)
        (`self.SetWindowOptions`)))))

(fn `IsWindowVisible`
  (returns (IsWindowVisible :type Boolean))
  (return (`self.IsVisible`)))

(fn `SetCollision`
  (params (InCollisionType :type "ECollisionEnabled Enum" :default "NoCollision") (InCollisionResponse :type "ECollisionResponse Enum" :default "ECR_Ignore") (InCollisionChannel :type "ECollisionChannel Enum" :default "ECC_WorldStatic"))
  (bind _windowmesh (`self.WindowMesh`))
  (`PrimitiveComponent.SetCollisionEnabled` _windowmesh InCollisionType)
  (`PrimitiveComponent.SetCollisionEnabled` (`self.SelectionMesh`) InCollisionType)
  (`PrimitiveComponent.SetCollisionEnabled` (`self.CloseMesh`) InCollisionType)
  (`PrimitiveComponent.SetCollisionEnabled` (`self.WidgetDisplayed`) InCollisionType)
  (`PrimitiveComponent.SetCollisionResponseToAllChannels` _windowmesh InCollisionResponse)
  (`PrimitiveComponent.SetCollisionResponseToAllChannels` (`self.SelectionMesh`) InCollisionResponse)
  (`PrimitiveComponent.SetCollisionResponseToAllChannels` (`self.CloseMesh`) InCollisionResponse)
  (`PrimitiveComponent.SetCollisionResponseToAllChannels` (`self.WidgetDisplayed`) InCollisionResponse)
  (`PrimitiveComponent.SetCollisionObjectType` _windowmesh InCollisionChannel)
  (`PrimitiveComponent.SetCollisionObjectType` (`self.SelectionMesh`) InCollisionChannel)
  (`PrimitiveComponent.SetCollisionObjectType` (`self.CloseMesh`) InCollisionChannel)
  (`PrimitiveComponent.SetCollisionObjectType` (`self.WidgetDisplayed`) InCollisionChannel))

(fn `SetHoverState`
  (params (InHoverState :type "/Game/VRIntegrator/Blueprints/E_DockWindowHover Enum" :default "NewEnumerator0"))
  (if (not (`|EnumEquality` InHoverState (`self.HoverState`)))
    (set `self.HoverState` InHoverState)
    (`self.UpdateHoverState`)))

(fn `SetupComponents`
  (params (InitResolution :type "Vector2D Structure" :default (1920.0 1080.0)) (InitScale :type "Float (double-precision)" :default 1.0) (UMGWidgetClass :type "UserWidget Class Reference"))
  (`|ExecutionSequence`
    (:`then_0`
      ;[1 1 1] Set the UMG resolution, this must remain high or widgets will get pixelated
      (set `self.Resolution` InitResolution)
      (set `self.Scale` InitScale)
      (`WidgetComponent.SetDrawSize` (`self.WidgetDisplayed`) (`self.Resolution`)))
    (:`then_1`
      ;[1 1 1] Inverse compensate for the window mesh initially
      (bind _outsize (`self.GetSize`))
      (bind (_x _y) (`KismetMathLibrary.BreakVector2D` (/ _outsize (`self.WindowMeshImportedSize`))))
      (`SceneComponent.SetRelativeScale3D` (`self.WindowMesh`) (`KismetMathLibrary.MakeVector` 1.0 _x _y)))
    (:`then_2`
      ;[1 1 1] Create the UMG widget and assign it to our Widget Component
      (bind _returnvalue (`|CreateWidget` UMGWidgetClass))
      (`WidgetComponent.SetWidget` (`self.WidgetDisplayed`) _returnvalue))))

(fn `SetWindowOptions`
  (`|ExecutionSequence`
    (:`then_0`
      ;[1 1 1] Setup Window Options
      (`SceneComponent.SetVisibility` (`self.CloseMesh`) (`self.IsClosable`) false)
      (`SceneComponent.SetVisibility` (`self.SelectionMesh`) (`self.IsMovable`) false)
      (`SceneComponent.SetVisibility` (`self.WindowMesh`) (`self.IsFramed`) false))
    (:`then_1`
      (if (not (`self.IsClosable`))
        (`PrimitiveComponent.SetCollisionEnabled` (`self.CloseMesh`) "NoCollision")))
    (:`then_2`
      (if (not (`self.IsMovable`))
        (`PrimitiveComponent.SetCollisionEnabled` (`self.SelectionMesh`) "NoCollision")))
    (:`then_3`
      (if (not (`self.IsFramed`))
        (`PrimitiveComponent.SetCollisionEnabled` (`self.WindowMesh`) "NoCollision")))))

(fn `ShowDockableWindow`
  (params (Show :type Boolean) (ForceUpdate :type Boolean))
  (if (not (and (not ForceUpdate) (== Show (`self.IsVisible`))))
    (bind _output_get (set `self.IsVisible` Show))
    (`self.SetActorHiddenInGame` (not _output_get))
    (if (`self.IsVisible`)
      (`self.SetCollision` "QueryOnly" "ECR_Block" "ECC_WorldDynamic")
      (else
        (`self.SetCollision` "NoCollision" "ECR_Ignore" "ECC_WorldDynamic")))))

(fn `UpdateHoverState`
  (bind _colorhovered (`self.ColorHovered`))
  (bind _colornormal (`self.ColorNormal`))
  (bind _colornormal_2 (`self.ColorNormal`))
  (bind _colorhovered_2 (`self.ColorHovered`))
  (bind _colornormal_3 (`self.ColorNormal`))
  (switch `/Game/VRIntegrator/Blueprints/E_DockWindowHover` (`self.HoverState`)
    (:`NewEnumerator0`
      (`MaterialInstanceDynamic.SetVectorParameterValue` (`self.MIDSelectionBar`) "Color" _colorhovered)
      (`MaterialInstanceDynamic.SetVectorParameterValue` (`self.MIDSelectionBarTranslucent`) "Color" _colorhovered)
      (`MaterialInstanceDynamic.SetVectorParameterValue` (`self.MIDCloseButton`) "Color" _colornormal)
      (`MaterialInstanceDynamic.SetVectorParameterValue` (`self.MIDCloseButtonTranslucent`) "Color" _colornormal))
    (:`NewEnumerator1`
      (`MaterialInstanceDynamic.SetVectorParameterValue` (`self.MIDSelectionBar`) "Color" _colornormal_2)
      (`MaterialInstanceDynamic.SetVectorParameterValue` (`self.MIDSelectionBarTranslucent`) "Color" _colornormal_2)
      (`MaterialInstanceDynamic.SetVectorParameterValue` (`self.MIDCloseButton`) "Color" _colorhovered_2)
      (`MaterialInstanceDynamic.SetVectorParameterValue` (`self.MIDCloseButtonTranslucent`) "Color" _colorhovered_2))
    (:`NewEnumerator2`
      (`MaterialInstanceDynamic.SetVectorParameterValue` (`self.MIDSelectionBar`) "Color" _colornormal_3 :!label _label)
      (`MaterialInstanceDynamic.SetVectorParameterValue` (`self.MIDSelectionBarTranslucent`) "Color" _colornormal_3)
      (`MaterialInstanceDynamic.SetVectorParameterValue` (`self.MIDCloseButton`) "Color" _colornormal_3)
      (`MaterialInstanceDynamic.SetVectorParameterValue` (`self.MIDCloseButtonTranslucent`) "Color" _colornormal_3))
    (:`NewEnumerator3`
      (goto _label))
    (:`NewEnumerator4`
      (goto _label))))

(fn `UpdateWindowMeshTransforms`
  (locals (Size :type "Vector2D Structure") (SelectionBarSize :type "Vector Structure") (CloseButtonSize :type "Vector Structure"))
  (bind _scale (`self.Scale`))
  (bind _x (`KismetMathLibrary.BreakVector2D` (`local.Size`)))
  (bind (_x_2 _y) (`KismetMathLibrary.BreakVector2D` (`local.Size`)))
  (bind _x_3 (`KismetMathLibrary.BreakVector2D` (`local.Size`)))
  (bind (_x_4 _y_2) (`KismetMathLibrary.BreakVector2D` (`local.Size`)))
  (bind (_x_5 _y_3) (`KismetMathLibrary.BreakVector2D` (`self.Resolution`)))
  (bind (_x_6 _y_4) (`KismetMathLibrary.BreakVector2D` (/ (`local.Size`) (`self.WindowMeshImportedSize`))))
  (`|ExecutionSequence`
    (:`then_0`
      (bind _outsize (`self.GetSize`))
      (set `local.Size` _outsize)
      (`SceneComponent.SetRelativeScale3D` (`self.WindowMesh`) (`KismetMathLibrary.MakeVector` 1.0 _x_6 _y_4)))
    (:`then_1`
      ;[1 1 1] Calculate size for UMG Wiget Component to be displayed and keep the desired resolution
      (`SceneComponent.SetWorldScale3D` (`self.WidgetDisplayed`) (* (`KismetMathLibrary.MakeVector` (/ 1.0 (`self.Scale`)) (/ 1.0 _x_5) (/ (/ 1.0 _y_3) (/ _x_5 _y_3))) (`KismetMathLibrary.MakeVector` _scale _scale _scale))))
    (:`then_2`
      ;[1 1 1] Size up the Selection Bar Mesh to match the window frame
      (bind _output_get (set `local.SelectionBarSize` (`KismetMathLibrary.MakeVector` 30.0 (* _x_3 0.8) (* _x_3 0.1))))
      (`SceneComponent.SetRelativeScale3D` (`self.SelectionMesh`) _output_get)
      (if (`self.IsClosable`)
        ;[1 1 1] Position the Selection Bar Mesh to line up with the window frame
        (`SceneComponent.K2_SetRelativeLocation` (`self.SelectionMesh`) (`KismetMathLibrary.MakeVector` 4.0 (- (* _x_4 0.5) (* (.y (`local.SelectionBarSize`)) 0.5)) (* (+ (* _y_2 0.5) (.z (`local.SelectionBarSize`)) (`self.SelectionBarOffset`)) -1.0)) false false)
        (else
          ;[1 1 1] Position the Selection Bar Mesh to line up with the window frame  without the close button
          (`SceneComponent.K2_SetRelativeLocation` (`self.SelectionMesh`) (`KismetMathLibrary.MakeVector` 4.0 0.0 (* (+ (* (`.Y` (`KismetMathLibrary.BreakVector2D` (`local.Size`))) 0.5) (.z (`local.SelectionBarSize`)) (`self.SelectionBarOffset`)) -1.0)) false false))))
    (:`then_3`
      ;[1 1 1] Scale and Position the Close Mesh correctly near the window
      (bind _output_get_2 (set `local.CloseButtonSize` (`KismetMathLibrary.MakeVector` 20.0 (* _x 0.1) (* _x 0.1))))
      (`SceneComponent.SetRelativeScale3D` (`self.CloseMesh`) _output_get_2)
      (`SceneComponent.K2_SetRelativeLocation` (`self.CloseMesh`) (`KismetMathLibrary.MakeVector` 4.0 (* (- (* _x_2 0.5) (* (.y (`local.CloseButtonSize`)) 0.5)) -1.0) (* (+ (* _y 0.5) (.z (`local.CloseButtonSize`)) (`self.SelectionBarOffset`)) -1.0)) false false))))

(fn `UserConstructionScript`
  (`self.SetupComponents` (`self.ResolutionUMG`) (`self.WindowScale`) (`self.UMGClass`))
  (`self.UpdateWindowMeshTransforms`)
  (`self.SetWindowOptions`)
  (`WidgetComponent.RequestRedraw` (`self.WidgetDisplayed`)))