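; A skeletal-mesh sword grabbable for VR hands, with a readiness flag that reports whether it can be grabbed.
; Grab stops physics, snaps the sword to the hand socket, clears its outline and swaps the hand to a left or right sword-grip AnimBP.
; Release restores the default hand AnimBP, detaches and re-enables physics.
; CollisionHeld is active only while held, but its overlap handler is empty.
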(event `self.ReceiveBeginPlay`
  (add `PrimitiveComponent.OnComponentBeginOverlap` (`self.CollisionHeld`) (delegate `OnComponentBeginOverlap_Event_0`))
  (`PrimitiveComponent.SetCollisionEnabled` (`self.CollisionHeld`) "NoCollision"))

(event `OnComponentBeginOverlap_Event_0`
  (params (OverlappedComponent :type "PrimitiveComponent Object Reference") (OtherActor :type "Actor Object Reference") (OtherComp :type "PrimitiveComponent Object Reference") (OtherBodyIndex :type Integer) (bFromSweep :type Boolean) (SweepResult :type "HitResult Structure (by ref)")))

(event `/Game/VRIntegrator/Blueprints/I_Grabbable.Grab`
  (params (AttachTo :type "SceneComponent Object Reference") (SocketName :type Name) (Hand :type "EControllerHand Enum" :default "Left"))
  (`|ExecutionSequence`
    (:`then_0`
      (set `self.Hand` Hand)
      (`PrimitiveComponent.SetSimulatePhysics` (`self.SkeletalMeshComponent`) false)
      (`SceneComponent.K2_AttachToComponent` (`self.RootComponent`) AttachTo SocketName "SnapToTarget" "SnapToTarget" "SnapToTarget" true)
      (`/Game/VRIntegrator/Blueprints/I_Grabbable.SetOutline` false)
      (`PrimitiveComponent.SetCollisionEnabled` (`self.CollisionHeld`) "QueryAndPhysics"))
    (:`then_1`
      (bind _asskeletal_mesh_component (cast `SkeletalMeshComponent` AttachTo))
      (if (`|EnumEquality` (`self.Hand`) "Left")
        (`SkeletalMeshComponent.SetAnimInstanceClass` _asskeletal_mesh_component "/Game/VRIntegrator/EpicContent/Hands/Left/AnimBP_L_SwordBones.AnimBP_L_SwordBones_C")
        (else
          (`SkeletalMeshComponent.SetAnimInstanceClass` _asskeletal_mesh_component "/Game/VRIntegrator/EpicContent/Hands/Right/AnimBP_R_SwordBones.AnimBP_R_SwordBones_C"))))))

(event `/Game/VRIntegrator/Blueprints/I_Grabbable.SetOutline`
  (params (InEnable :type Boolean) (InStencil :type Integer))
  (bind _skeletalmeshcomponent (`self.SkeletalMeshComponent`))
  (`PrimitiveComponent.SetCustomDepthStencilValue` _skeletalmeshcomponent InStencil)
  (`PrimitiveComponent.SetRenderCustomDepth` _skeletalmeshcomponent InEnable))

(event `/Game/VRIntegrator/Blueprints/I_Grabbable.Release`
  (`|ExecutionSequence`
    (:`then_0`
      (bind _asskeletal_mesh_component (cast `SkeletalMeshComponent` (`SceneComponent.GetAttachParent` (`self.SkeletalMeshComponent`))))
      (if (`|EnumEquality` (`self.Hand`) "Left")
        (`SkeletalMeshComponent.SetAnimInstanceClass` _asskeletal_mesh_component "/Game/VRIntegrator/EpicContent/Hands/Left/AnimBP_L_Hand_Def.AnimBP_L_Hand_Def_C")
        (else
          (`SkeletalMeshComponent.SetAnimInstanceClass` _asskeletal_mesh_component "/Game/VRIntegrator/EpicContent/Hands/Right/AnimBP_R_Hand_Def.AnimBP_R_Hand_Def_C"))))
    (:`then_1`
      (`PrimitiveComponent.SetSimulatePhysics` (`self.SkeletalMeshComponent`) true)
      (`self.K2_DetachFromActor` "KeepWorld" "KeepWorld" "KeepWorld")
      (`PrimitiveComponent.SetCollisionEnabled` (`self.CollisionHeld`) "NoCollision"))))

(event `/Game/VRIntegrator/Blueprints/I_Grabbable.SetGrabbaleEnabled`
  (params (Enabled :type Boolean))
  (set `self.IsReadyForGrab` Enabled))

(fn `CanBeGrabbed`
  (returns (IsGrabbableReady :type Boolean))
  (return (`self.IsReadyForGrab`)))

(fn `UserConstructionScript`)