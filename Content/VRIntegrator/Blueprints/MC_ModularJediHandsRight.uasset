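; MC_ModularJediHandsRight is a VR motion controller for the right hand, combining a Jedi hand ability with a smoothed laser pointer and teleport.
; On BeginPlay it initializes both child actors with the hand, pawn and motion controller.
; Grip input drives the Jedi hand, while trigger and thumbstick input drive the laser.
; After creation it registers laser ignore lists against the left controller, its child actors and actors tagged TeleportIgnored.
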(event `self.ReceiveBeginPlay`
  (bind _smoothlaser (`self.SmoothLaser`))
  (`parent.ReceiveBeginPlay`)
  (set `MotionControllerComponent.Hand` (`self.Hand`) (`self.MotionController`))
  (`|ExecutionSequence`
    (:`then_0`
      (bind _asca_jedi_hands_right (cast `/Game/VRIntegrator/ChildActors/CA_JediHandsRight` (`ChildActorComponent.ChildActor` (`self.ChildJediHands`))))
      (bind _output_get (set `self.JediHand` _asca_jedi_hands_right))
      (`/Game/VRIntegrator/ChildActors/CA_JediHandsRight.Initialize` _output_get (`self.Hand`) (`self.ParentVRBasePawn`) (`self.MotionController`))
      (set `/Game/VRIntegrator/ChildActors/CA_JediHandsRight.CanJediAbility` true (`self.JediHand`)))
    (:`then_1`
      (bind _asca_smoothed_laser (cast `/Game/VRIntegrator/ChildActors/CA_SmoothedLaser` (`ChildActorComponent.ChildActor` (`self.ChildSmoothLaser`))))
      (bind _output_get_2 (set `self.SmoothLaser` _asca_smoothed_laser))
      (`/Game/VRIntegrator/ChildActors/CA_SmoothedLaser.Initialize` _output_get_2 (`self.Hand`) (`self.ParentVRBasePawn`) (`self.MotionController`))
      (set `/Game/VRIntegrator/ChildActors/CA_SmoothedLaser.CanLaserPointer` true _smoothlaser)
      (set `/Game/VRIntegrator/ChildActors/CA_SmoothedLaser.CanTeleport` true _smoothlaser)
      (`/Game/VRIntegrator/ChildActors/CA_SmoothedLaser.Activate` _smoothlaser true)
      (`KismetArrayLibrary.Array_Add` (`/Game/VRIntegrator/ChildActors/CA_SmoothedLaser.ActorsToIgnore` _smoothlaser) (`self.JediHand`)))))

(event `self.OnPostCreation`
  (`self.RegisterExternalIgnoredActors` (`/Game/VRIntegrator/Blueprints/BP_VRBasePawn.LeftHandController` (`self.ParentVRBasePawn`))))

(event `self.InputTriggerPressed`
  (bind _smoothlaser (`self.SmoothLaser`)
    (:`then`
      (`/Game/VRIntegrator/ChildActors/CA_SmoothedLaser.OnTriggerPressed` _smoothlaser))
    (:`else`)))

(event `self.SetupControllerMesh`
  (params (InMeshComponent :type "SceneComponent Object Reference"))
  (`parent.SetupControllerMesh` InMeshComponent))

(event `self.InputTriggerReleased`
  (bind _smoothlaser (`self.SmoothLaser`)
    (:`then`
      (`/Game/VRIntegrator/ChildActors/CA_SmoothedLaser.OnTriggerReleased` _smoothlaser))
    (:`else`)))

(event `self.ReceiveTick`
  (params (DeltaSeconds :type "Float (single-precision)"))
  (`parent.ReceiveTick` DeltaSeconds)
  (bind _smoothlaser (`self.SmoothLaser`)
    (:`then`
      (`/Game/VRIntegrator/ChildActors/CA_SmoothedLaser.UpdateThumbstick` _smoothlaser (`self.ThumbstickUpAxis`) (`self.ThumbstickRightAxis`)))
    (:`else`)))

(event `self.InputGrip1Pressed`
  (bind _jedihand (`self.JediHand`)
    (:`then`
      (`/Game/VRIntegrator/ChildActors/CA_JediHandsRight.OnGripPressed` _jedihand))
    (:`else`)))

(event `self.InputGrip1Released`
  (bind _jedihand (`self.JediHand`)
    (:`then`
      (`/Game/VRIntegrator/ChildActors/CA_JediHandsRight.OnGripReleased` _jedihand))
    (:`else`)))

(fn `RegisterExternalIgnoredActors`
  (params (InBaseMotionController :type "/Game/VRIntegrator/Blueprints/BP_BaseMotionController Object Reference"))
  (bind _childactors (`self.GetAllChildActors` InBaseMotionController true))
  (bind _actorstoignore (`/Game/VRIntegrator/ChildActors/CA_SmoothedLaser.ActorsToIgnore` (`self.SmoothLaser`)))
  (`|ExecutionSequence`
    (:`then_0`
      (`/Engine/EditorBlueprintResources/StandardMacros.IsValid` InBaseMotionController
        (:`Is Valid`
          (`KismetArrayLibrary.Array_Add` _actorstoignore InBaseMotionController)
          (`KismetArrayLibrary.Array_Append` _actorstoignore _childactors)
          (for _array_element _childactors
            (bind _asca_smoothed_laser (cast `/Game/VRIntegrator/ChildActors/CA_SmoothedLaser` _array_element))
            (bind _actorstoignore_2 (`/Game/VRIntegrator/ChildActors/CA_SmoothedLaser.ActorsToIgnore` _asca_smoothed_laser))
            (`KismetArrayLibrary.Array_AddUnique` _actorstoignore_2 (`self.SmoothLaser`))
            (`KismetArrayLibrary.Array_AddUnique` _actorstoignore_2 (`self.JediHand`))))))
    (:`then_1`
      (bind _outactors (`GameplayStatics.GetAllActorsWithTag` "TeleportIgnored"))
      (`KismetArrayLibrary.Array_Append` (`/Game/VRIntegrator/ChildActors/CA_SmoothedLaser.ActorsToIgnore` (`self.SmoothLaser`)) _outactors))))

(fn `UserConstructionScript`
  (`parent.UserConstructionScript`))